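; Editor tool actor that scatters randomly chosen static meshes onto surfaces found by line traces.
; ScatterObjects picks random points along ScatterSize's right and up axes, without adding a world position, and traces along SpawnDirection with debug drawing.
; Each hit spawns a randomly scaled StaticMeshActor with a mesh from MeshesToSpawn.
; The construction script scales ScatterSize to PlaneSize.
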(event Custom|ScatterObjects
  (bind _scattersize (Variables|Default|GetScatterSize))
  (bind _planesize (Variables|Default|GetPlaneSize))
  (for _index (range 0 (- (Variables|Default|GetNumObjects) 1))
    (bind _output_get (Variables|Default|SetRayStart (+ (* (Math|Vector|GetRightVector _scattersize) (Math|Random|RandomFloatinRange (* (.x _planesize) -1.0) (.x _planesize))) (* (Math|Vector|GetUpVector _scattersize) (Math|Random|RandomFloatinRange (* (.y _planesize) -1.0) (.y _planesize))))))
    (Variables|Default|SetRayEnd (+ _output_get (* (Math|Vector|GetForwardVector (Variables|Default|GetSpawnDirection)) 5e+02)))
    (bind (_outhit _returnvalue) (Collision|LineTraceByChannel (Variables|Default|GetRayStart) (Variables|Default|GetRayEnd) "TraceTypeQuery4" false 0 "ForDuration"))
    (if _returnvalue
      (bind _returnvalue_2 (Game|SpawnActorfromClass "/Script/Engine.StaticMeshActor" (Math|Transform|MakeTransform (.Location (Collision|BreakHitResult _outhit)) "0, 0, 0" (Math|Conversions|ToVector(Float) (+ (* (Math|Random|RandomFloat) 1.0) 0.5))) "AdjustIfPossibleButAlwaysSpawn" 0 0))
      (Utilities|IsValid _returnvalue_2
        (:Is%20Valid
          (Components|StaticMesh|SetStaticMesh (Variables|/Script/Engine.StaticMeshActor|GetStaticMeshComponent _returnvalue_2) (.OutItem (Utilities|Array|Random (Variables|Default|GetMeshesToSpawn)))))))))

(fn ConstructionScript
  (bind _planesize (Variables|Default|GetPlaneSize))
  (Transformation|SetWorldScale3D (Variables|Default|GetScatterSize) (Math|Vector|MakeVector (.x _planesize) (.y _planesize) 0.0)))