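; BP_RockActorBase is a base Blueprint for LucidWorld rock actors that hooks them up to the LucidVisibility system.
; On BeginPlay it calls OnVisibilityChanged with the current IsVisible state, then binds to LucidVisibility's visibility-changed delegate before calling the parent.
; OnVisibilityChanged is empty here, so the base only supplies the wiring and has no visibility response of its own.
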(event Custom|OnVisibilityChanged
  (params (NewVisibility :type Boolean)))

(event EventBeginPlay
  (bind _lucidvisibility (Variables|Default|GetLucidVisibility))
  (CallFunction|OnVisibilityChanged (Variables|/Script/Lucido.LucidVisibilityComponent|GetbIsVisible _lucidvisibility))
  (EventDispatchers|BindEventtoOnVisibilityChangedDelegate _lucidvisibility (EventDispatchers|CreateEvent :!event Custom|OnVisibilityChanged))
  (|CallParentFunction))

(event Collision|EventActorBeginOverlap
  (params (OtherActor :type Actor%20Object%20Reference))
  (|CallParentFunction OtherActor) ; This node is disabled and will not be called.\nDrag off pins to build functionality.
)

(event EventTick
  (params (DeltaSeconds :type Float%20%28single-precision%29))
  (|CallParentFunction DeltaSeconds) ; This node is disabled and will not be called.\nDrag off pins to build functionality.
)

(fn ConstructionScript
  (|CallParentFunction))