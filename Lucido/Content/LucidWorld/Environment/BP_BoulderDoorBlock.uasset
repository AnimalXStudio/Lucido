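; BP_BoulderDoorBlock is a boulder obstacle, apparently a door blocker, whose solidity follows its lucid visibility state.
; On BeginPlay it applies the current MLucidVisibilityComponent visibility and binds to that component's visibility-changed delegate.
; The handler gives Rocks query and physics collision when visible and none when hidden.
; Starting an interaction only sends an interaction-failed message.
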(event Custom|OnVisibilityChanged
  (params (NewVisibility :type Boolean))
  (Collision|SetCollisionEnabled (Variables|Default|GetRocks) (select NewVisibility "QueryAndPhysics" "NoCollision")))

(event EventBeginPlay
  (bind _m_lucidvisibilitycomponent (Variables|Default|Getm_LucidVisibilityComponent))
  (CallFunction|OnVisibilityChanged (Variables|/Script/Lucido.LucidVisibilityComponent|GetbIsVisible _m_lucidvisibilitycomponent))
  (EventDispatchers|BindEventtoOnVisibilityChangedDelegate _m_lucidvisibilitycomponent (EventDispatchers|CreateEvent :!event Custom|OnVisibilityChanged))
  (|CallParentFunction))

(event Collision|EventActorBeginOverlap
  (params (OtherActor :type Actor%20Object%20Reference))
  (|CallParentFunction OtherActor) ; This node is disabled and will not be called.\nDrag off pins to build functionality.
)

(event EventTick
  (params (DeltaSeconds :type Float%20%28single-precision%29))
  (|CallParentFunction DeltaSeconds) ; This node is disabled and will not be called.\nDrag off pins to build functionality.
)

(event EventInteractionStarted
  (params (TargetingCharacter :type Lucid%20Character%20Object%20Reference))
  (Class|LucidToolBase|SendonInteractionFailedMessage 6.0))

(fn ConstructionScript
  (|CallParentFunction))